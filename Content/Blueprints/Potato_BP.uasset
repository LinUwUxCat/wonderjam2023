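; Potato_BP is a physics-simulated potato projectile that can be thrown and sent back toward a player position.
; Throw sets the capsule's linear velocity, while GetBackToPlayer switches collision to OverlapAll, disables gravity and flies straight at the given position at fixed speed.
; Tick counts down a timer to spawn PotatoSmoke actors at short intervals as a trail, slightly offset from the potato.
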(event `self.ReceiveActorBeginOverlap`
  (params (OtherActor :type "Actor Object Reference")))

(event `Throw`
  (params (velocity :type "Vector Structure"))
  (`PrimitiveComponent.SetAllPhysicsLinearVelocity` (`self.CapsuleComponent`) velocity false))

(event `self.ReceiveTick`
  (params (DeltaSeconds :type "Float (single-precision)"))
  (bind _output_get (set `self.nextSmokeIn` (- (`self.nextSmokeIn`) DeltaSeconds)))
  (if (<= _output_get 0.0)
    (set `self.nextSmokeIn` 0.2)
    (`|SpawnActorFromClass` "/Game/Blueprints/PotatoSmoke.PotatoSmoke_C" (`KismetMathLibrary.MakeTransform` (`KismetMathLibrary.MakeVector` (.x (.location (`self.GetTransform`))) (- (.y (.location (`self.GetTransform`))) 0.2) (.z (.location (`self.GetTransform`)))) (.rotation (`self.GetTransform`)) (.scale (`self.GetTransform`))) "Undefined" "MultiplyWithRoot" null null)))

(fn `GetBackToPlayer`
  (params (Position :type "Vector Structure"))
  (bind _capsulecomponent (`self.CapsuleComponent`))
  (`PrimitiveComponent.SetCollisionProfileName` _capsulecomponent "OverlapAll" true)
  (`PrimitiveComponent.SetEnableGravity` _capsulecomponent false)
  (`PrimitiveComponent.SetAllPhysicsLinearVelocity` _capsulecomponent (* (`KismetMathLibrary.Normal` (- Position (`self.K2_GetActorLocation`))) 600) false))

(fn `UserConstructionScript`
  (`PrimitiveComponent.SetSimulatePhysics` (`self.CapsuleComponent`) true)
  (set `self.nextSmokeIn` 0.2))