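; Door actor that shows a tile map sprite with a designer-chosen color and size.
; The construction script maps the Color enum to a blue, red or green tint, leaving grey unchanged, and applies it to the tile map component.
; It clamps Size to one or two and uses GetTileMap to pick the 1x1 or 1x2 door tile map.
; The event graph has no logic.
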(fn `Get Tile Map`
  (returns (TileMap :type "PaperTileMap Object Reference"))
  (if (== 1 (`self.size`))
    (return "/Game/Sprites/door1x1.door1x1")
    (else
      (return "/Game/Sprites/door1x2.door1x2"))))

(fn `UserConstructionScript`
  (switch `/Game/Blueprints/ButtonColor` (`self.Color`)
    (:`NewEnumerator0`
      (`KismetMathLibrary.LinearColor_SetRGBA` (`self.currentColor`) 0.0 0.0 1.0))
    (:`NewEnumerator1`
      (`KismetMathLibrary.LinearColor_SetRGBA` (`self.currentColor`) 1.0))
    (:`NewEnumerator2`
      _)
    (:`NewEnumerator3`
      (`KismetMathLibrary.LinearColor_SetRGBA` (`self.currentColor`) 0.0 1.0)))
  (`PaperTileMapComponent.SetTileMapColor` (`self.RenderComponent`) (`self.currentColor`))
  (set `self.size` (`KismetMathLibrary.Clamp` (`self.size`) 1 2))
  (bind _tilemap (`self.Get Tile Map`))
  (`PaperTileMapComponent.SetTileMap` (`self.RenderComponent`) _tilemap))