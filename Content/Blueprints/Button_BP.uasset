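; A coloured tile-map pressure button that opens its linked Door while the main character or a potato actor stands on it.
; Overlap events count those actors, and Tick hides the Door and disables its collision while any are present.
; Tick also swaps the pressed or released tile map by Color, though the construction script previews only blue or red.
; An InverseBehavior flag can flip the door logic, but BeginPlay resets it to false.
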(event `self.ReceiveBeginPlay`
  (set `self.overlappingObjects` 0)
  (set `self.inverseBehavior` false))

(event `self.ReceiveActorBeginOverlap`
  (params (OtherActor :type "Actor Object Reference"))
  (if (or (`GameplayStatics.ObjectIsA` OtherActor "/Game/Character/BP_MainCharacter.BP_MainCharacter_C") (`GameplayStatics.ObjectIsA` OtherActor "/Game/Blueprints/Potato_BP.Potato_BP_C"))
    (`/Engine/EditorBlueprintResources/StandardMacros.IncrementInt` (`self.overlappingObjects`))))

(event `self.ReceiveActorEndOverlap`
  (params (OtherActor :type "Actor Object Reference"))
  (if (or (`GameplayStatics.ObjectIsA` OtherActor "/Game/Character/BP_MainCharacter.BP_MainCharacter_C") (`GameplayStatics.ObjectIsA` OtherActor "/Game/Blueprints/Potato_BP.Potato_BP_C"))
    (`/Engine/EditorBlueprintResources/StandardMacros.DecrementInt` (`self.overlappingObjects`))))

(event `self.ReceiveTick`
  (params (DeltaSeconds :type "Float (single-precision)"))
  (bind _door (`self.Door`))
  (bind _returnvalue (!= (`self.overlappingObjects`) 0))
  (bind _returnvalue_2 (xor _returnvalue (`self.inverseBehavior`)))
  (`self.SetActorHiddenInGame` _door _returnvalue_2)
  (`self.SetActorEnableCollision` _door (not _returnvalue_2))
  (bind _tilemap (`self.GetTileMap` _returnvalue))
  (`PaperTileMapComponent.SetTileMap` (`self.RenderComponent`) _tilemap))

(fn `GetTileMap`
  (params (Pressed :type Boolean))
  (returns (TileMap :type "PaperTileMap Object Reference"))
  (bind _color (`self.Color`))
  (if Pressed
    (switch `/Game/Blueprints/ButtonColor` _color
      (:`NewEnumerator0`
        (return "/Game/Sprites/Buttons/BluePressed_TileMap.BluePressed_TileMap"))
      (:`NewEnumerator1`
        (return "/Game/Sprites/Buttons/RedPressed_TileMap.RedPressed_TileMap"))
      (:`NewEnumerator2`
        (return "/Game/Sprites/Buttons/GreyPressed_TileMap.GreyPressed_TileMap"))
      (:`NewEnumerator3`
        (return "/Game/Sprites/Buttons/GreenPressed_TileMap.GreenPressed_TileMap")))
    (else
      (switch `/Game/Blueprints/ButtonColor` _color
        (:`NewEnumerator0`
          (return "/Game/Sprites/Buttons/Blue_TileMap.Blue_TileMap"))
        (:`NewEnumerator1`
          (return "/Game/Sprites/Buttons/Red_TileMap.Red_TileMap"))
        (:`NewEnumerator2`
          (return "/Game/Sprites/Buttons/Grey_TileMap.Grey_TileMap"))
        (:`NewEnumerator3`
          (return "/Game/Sprites/Buttons/Green_TileMap.Green_TileMap"))))))

(fn `UserConstructionScript`
  (if (`|EnumEquality` "NewEnumerator0" (`self.Color`))
    (`PaperTileMapComponent.SetTileMap` (`self.RenderComponent`) "/Game/Sprites/BtnBlue.BtnBlue")
    (else
      (if (`|EnumEquality` "NewEnumerator1" (`self.Color`))
        _
        (else
          _))
      (`PaperTileMapComponent.SetTileMap` (`self.RenderComponent`) "/Game/Sprites/BtnRed.BtnRed"))))