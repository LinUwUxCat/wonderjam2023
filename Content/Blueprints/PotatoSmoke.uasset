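; PotatoSmoke is a short-lived 2D smoke puff actor that drifts and fades out.
; The construction script picks one of five smoke sprites at random for the render component.
; On BeginPlay it enables physics without gravity and sets a random, mostly upward velocity in the XZ plane.
; Tick counts down a two-second lifetime, lowering sprite alpha in proportion until the actor destroys itself.
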(event `self.ReceiveBeginPlay`
  (bind _rendercomponent (`self.RenderComponent`))
  (set `self.timeToLive` 2.0)
  (`PrimitiveComponent.SetSimulatePhysics` _rendercomponent true)
  (`PrimitiveComponent.SetEnableGravity` _rendercomponent false)
  (`PrimitiveComponent.SetAllPhysicsLinearVelocity` _rendercomponent (`KismetMathLibrary.MakeVector` (`KismetMathLibrary.RandomFloatInRange` -10.0 10.0) 0.0 (`KismetMathLibrary.RandomFloatInRange` -1.0 30.0)) false))

(event `self.ReceiveTick`
  (params (DeltaSeconds :type "Float (single-precision)"))
  (bind _output_get (set `self.timeToLive` (- (`self.timeToLive`) DeltaSeconds)))
  (if (<= _output_get 0.0)
    (`self.K2_DestroyActor`)
    (else
      (`PaperSpriteComponent.SetSpriteColor` (`self.RenderComponent`) (make `LinearColor` 1.0 1.0 1.0 (/ _output_get 2.0))))))

(fn `UserConstructionScript`
  (switch `int` (`KismetMathLibrary.RandomIntegerInRange` 1 5)
    (:`1`
      (set `self.startingSprite` "/Game/Sprites/Smoke1_Sprite.Smoke1_Sprite"))
    (:`2`
      (set `self.startingSprite` "/Game/Sprites/Smoke2_Sprite.Smoke2_Sprite"))
    (:`3`
      (set `self.startingSprite` "/Game/Sprites/Smoke3_Sprite.Smoke3_Sprite"))
    (:`4`
      (set `self.startingSprite` "/Game/Sprites/Smoke4_Sprite.Smoke4_Sprite"))
    (:`5`
      (set `self.startingSprite` "/Game/Sprites/Smoke5_Sprite.Smoke5_Sprite")))
  (`PaperSpriteComponent.SetSprite` (`self.RenderComponent`) (`self.startingSprite`)))