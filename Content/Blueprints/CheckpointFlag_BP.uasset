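; Checkpoint flag actor that sets the main character's respawn point on contact.
; When BP_MainCharacter begins overlapping the box collision, the render component switches its flipbook to the USA flag.
; It then writes the character's Respawn transform from the box's world location, raised along Z, and the box's rotation, with unit scale.
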(event `self.BoxCollision.OnComponentBeginOverlap`
  (params (OverlappedComponent :type "PrimitiveComponent Object Reference") (OtherActor :type "Actor Object Reference") (OtherComp :type "PrimitiveComponent Object Reference") (OtherBodyIndex :type Integer) (bFromSweep :type Boolean) (SweepResult :type "HitResult Structure (by ref)"))
  (if (`GameplayStatics.ObjectIsA` OtherActor "/Game/Character/BP_MainCharacter.BP_MainCharacter_C")
    (`PaperFlipbookComponent.SetFlipbook` (`self.RenderComponent`) "/Game/Sprites/Flags/USAFlag.USAFlag")
    (bind _asbp_main_character (cast `/Game/Character/BP_MainCharacter` OtherActor))
    (set `/Game/Character/BP_MainCharacter.Respawn` (`KismetMathLibrary.MakeTransform` (+ (.location (`SceneComponent.K2_GetComponentToWorld` (`self.BoxCollision`))) (0.0 0.0 150.0)) (.rotation (`SceneComponent.K2_GetComponentToWorld` (`self.BoxCollision`)))) _asbp_main_character)))

(fn `UserConstructionScript`)