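; Lever actor that toggles a linked Door when a Potato_BP enters its collision box.
; Each toggle hides or shows the Door with matching collision and swaps the sprite between left and right lever tile maps.
; It also sets InverseBehavior on every Button_BP sharing that Door to the new toggle state.
; A separate ReactivateBox re-arms the lever only after the potato leaves it, preventing repeated toggles.
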(event `self.ReceiveBeginPlay`
  (set `self.IsPotatoInRange` false))

(event `self.ReceiveTick`
  (params (DeltaSeconds :type "Float (single-precision)")))

(event `self.BoxCollision.OnComponentBeginOverlap`
  (params (OverlappedComponent :type "PrimitiveComponent Object Reference") (OtherActor :type "Actor Object Reference") (OtherComp :type "PrimitiveComponent Object Reference") (OtherBodyIndex :type Integer) (bFromSweep :type Boolean) (SweepResult :type "HitResult Structure (by ref)"))
  (if (`GameplayStatics.ObjectIsA` OtherActor "/Game/Blueprints/Potato_BP.Potato_BP_C")
    (if (not (`self.IsPotatoInRange`))
      (set `self.IsPotatoInRange` true)
      (bind _output_get (set `self.toggled` (not (`self.toggled`))))
      (`self.SetActorHiddenInGame` (`self.Door`) _output_get)
      (`self.SetActorEnableCollision` (`self.Door`) (not _output_get))
      (bind _tilemap (`self.GetTileMap`))
      (`PaperTileMapComponent.SetTileMap` (`self.RenderComponent`) _tilemap)
      (bind _outactors (`GameplayStatics.GetAllActorsOfClass` "/Game/Blueprints/Button_BP.Button_BP_C"))
      (for _array_element _outactors
        (if (== (`/Game/Blueprints/Button_BP.Door` _array_element) (`self.Door`))
          (set `/Game/Blueprints/Button_BP.inverseBehavior` (`self.toggled`) _array_element))))))

(event `self.ReactivateBox.OnComponentEndOverlap`
  (params (OverlappedComponent :type "PrimitiveComponent Object Reference") (OtherActor :type "Actor Object Reference") (OtherComp :type "PrimitiveComponent Object Reference") (OtherBodyIndex :type Integer))
  (if (`GameplayStatics.ObjectIsA` OtherActor "/Game/Blueprints/Potato_BP.Potato_BP_C")
    (set `self.IsPotatoInRange` false)))

(fn `GetTileMap`
  (returns (Tilemap :type "PaperTileMap Object Reference"))
  (if (`self.toggled`)
    (return "/Game/Sprites/LevierLeft.LevierLeft")
    (else
      (return "/Game/Sprites/LevierRight.LevierRight"))))

(fn `UserConstructionScript`)